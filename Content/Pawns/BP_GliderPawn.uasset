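; BP_GliderPawn is a glider pawn that drives wing-trail visuals and shows live flight debug info.
; Each tick it sets the TraceWidth of both wing Niagara traces from the mesh's forward pitch above a threshold, only when forward speed from the flight physics component is high enough.
; It also prints forward speed, dash stamina and current health on screen every frame.
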(event EventTick
  (params (DeltaSeconds :type Float%20%28single-precision%29))
  (bind _meshcomponent (Variables|Default|GetMeshComponent))
  (bind _wingtraceinclinationthreshold (Variables|Default|GetWingTraceInclinationThreshold))
  (bind _returnvalue (Math|Vector|GetForwardVector _meshcomponent))
  (bind _returnvalue_2 (Math|Float|Absolute(Float) (.z _returnvalue)))
  (|CallParentFunction 0.0)
  ;[1 1 1] Controls niagara visuals for wings traces. If inclination and speed conditions are met, trace will be visible.
  (Effects|Components|ParticleSystem|SetFloatParameter (Variables|Default|GetLeft%20Wing%20Trace) "TraceWidth" (select (and (> (Variables|/Script/ProjectFly.FlightPhysicsComponent|GetForwardSpeed (Variables|Default|GetFlightPhysicsComponent)) (Variables|Default|GetWingTraceSpeedThreshold)) (> _returnvalue_2 _wingtraceinclinationthreshold)) (- _returnvalue_2 _wingtraceinclinationthreshold) 0.0))
  (Development|PrintString (Utilities|String|ToString(Float) (Variables|/Script/ProjectFly.FlightPhysicsComponent|GetForwardSpeed (Variables|Default|GetFlightPhysicsComponent))) true true "(R=1.000000,G=0.072570,B=0.000000,A=1.000000)" 0.1)
  (Development|PrintString (Utilities|String|ToString(Float) (Variables|Default|GetCurrentDashStamina)) true true "(R=0.000000,G=0.660000,B=1.000000,A=1.000000)" 0.1)
  (Development|PrintString (Utilities|String|ToString(Float) (Variables|/Script/ProjectFly.HealthComponent|GetCurrentHealth (Variables|Default|GetHealthComponent))) true true "(R=0.251515,G=1.000000,B=0.000000,A=1.000000)" 0.1))

(fn ConstructionScript)