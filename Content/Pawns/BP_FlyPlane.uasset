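; BP_FlyPlane is a plane pawn Blueprint that drives the Niagara wingtrail visuals on its left and right wings.
; After calling the parent Tick, it updates the TraceWidth parameter on both trace components every frame.
; Traces show only when forward speed and nose pitch, read as the absolute Z of the forward vector, exceed their thresholds.
; Width grows with pitch beyond the threshold and is zero otherwise.
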(event EventTick
  (params (DeltaSeconds :type Float%20%28single-precision%29))
  (bind _returnvalue (Transformation|GetActorForwardVector))
  (bind _wingtraceinclinationthreshold (Variables|PlaneVisuals|GetWingTraceInclinationThreshold))
  (bind _returnvalue_2 (Math|Float|Absolute(Float) (.z _returnvalue)))
  (|CallParentFunction 0.0)
  ;[1 1 1] Controls niagara visuals for wings traces. If inclination and speed conditions are met, trace will be visible.
  (Effects|Components|ParticleSystem|SetFloatParameter (Variables|Default|GetLeft%20Wing%20Trace) "TraceWidth" (select (and (> (Variables|Default|GetForwardSpeed) (Variables|PlaneVisuals|GetWingTraceSpeedThreshold)) (> _returnvalue_2 _wingtraceinclinationthreshold)) (- _returnvalue_2 _wingtraceinclinationthreshold) 0.0)))

(fn ConstructionScript)