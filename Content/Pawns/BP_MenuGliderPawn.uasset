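; Glider pawn, named for use in the menu, that adds wing trace visuals on top of its parent's behavior.
; Each Tick calls the parent, then sets the TraceWidth parameter on the left and right Niagara wing traces.
; Traces show only when forward speed from FlightPhysicsComponent and mesh inclination (absolute forward-vector Z) both exceed thresholds.
; Width equals the inclination beyond its threshold, and zero otherwise.
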(event EventTick
  (params (DeltaSeconds :type Float%20%28single-precision%29))
  (bind _meshcomponent (Variables|Default|GetMeshComponent))
  (bind _wingtraceinclinationthreshold (Variables|Default|GetWingTraceInclinationThreshold))
  (bind _returnvalue (Math|Vector|GetForwardVector _meshcomponent))
  (bind _returnvalue_2 (Math|Float|Absolute(Float) (.z _returnvalue)))
  (|CallParentFunction 0.0)
  ;[1 1 1] Controls niagara visuals for wings traces. If inclination and speed conditions are met, trace will be visible.
  (Effects|Components|ParticleSystem|SetFloatParameter (Variables|Default|GetLeft%20Wing%20Trace) "TraceWidth" (select (and (> (Variables|/Script/ProjectFly.FlightPhysicsComponent|GetForwardSpeed (Variables|Default|GetFlightPhysicsComponent)) (Variables|Default|GetWingTraceSpeedThreshold)) (> _returnvalue_2 _wingtraceinclinationthreshold)) (- _returnvalue_2 _wingtraceinclinationthreshold) 0.0)))

(fn ConstructionScript)